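; Game instance that routes players to the options or main menu based on a save-file check and manages multiplayer sessions.
; Menu events create widgets and cache all but the server list, which is rebuilt each time.
; Hosting creates an Advanced Session tagged with the server name, then opens Lobby as a listen server; joining and destroying sessions are also wrapped here.
; Network and travel error handlers exist, but their string and display functions are empty stubs.
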(event Custom|ShowMainMenu
  (bind _returnvalue (Game|GetPlayerController 0))
  ;[1 1 1] 이미 메뉴가 있는지 확인
  ; 이미 있으면 만들었던 거 다시 띄움
  (Utilities|IsValid (Variables|Widgets|GetMainMenuWB)
    (:Is%20Valid
      _)
    (:Is%20Not%20Valid
      ;[1 1 1] 없으면 만들고 변수로 저장해둠
      (bind _returnvalue_2 (UserInterface|CreateWidget "/Game/UI/MainMenu/MainMenu.MainMenu_C" _returnvalue))
      (Variables|Widgets|SetMainMenuWB _returnvalue_2)))
  ;[1 1 1] 저장한 거 화면에 표시 후 마우스 커서 표시
  (UserInterface|Viewport|AddtoViewport (Variables|Widgets|GetMainMenuWB) 0)
  (Variables|/Script/Engine.PlayerController|SetbShowMouseCursor _returnvalue true))

(event Custom|LaunchLobby
  (params (NumberOfPlayer :type Integer) (isEnableLAN :type Boolean) (ServerName :type Text))
  ;[1 1 1] 호스트 설정으로 로비 열기 - 리슨 서버로 게임을 연다.
  ;[1 1 1] 호스트 설정으로 로비 열기 - 리슨 서버로 게임을 연다.
  (Variables|ServerSettings|SetMaxPlayers NumberOfPlayer)
  (bind _output_get (Variables|ServerSettings|SetServerName ServerName))
  (CallFunction|ShowLoadingScreen)
  (|AdvancedSession (Utilities|Array|MakeArray (Class|AdvancedSessionsLibrary|MakeLiteralSessionPropertyString "GAMENAME" (Utilities|String|ToString(Text) _output_get))) (Game|GetPlayerController 0) (Variables|ServerSettings|GetMaxPlayers) 0 isEnableLAN true false true true true false false false true false true ; Make an advanced session with the extra session properties
    (:OnSuccess
      (Game|OpenLevel(byName) "Lobby" false "listen"))
    (:OnFailure
      (Utilities|DisplayErrorMessage "Fail To Create Session"))))

(event Custom|JoinServer
  (params (SessionToJoin :type Blueprint%20Session%20Result%20Structure))
  ;[1 1 1] 서버 메뉴에서 서버 접속
  ;[1 1 1] 호스트 설정으로 로비 열기 - 리슨 서버로 게임을 연다.
  (Development|PrintString "Join Server")
  (CallFunction|ShowLoadingScreen)
  (|JoinSession (Game|GetPlayerController 0) SessionToJoin
    (:OnFailure
      (Utilities|DisplayErrorMessage "Fail to Join Session"))))

(event Custom|DestroySessionCaller
  (params (PlayerController :type AR%20Shared%20World%20Player%20Controller%20Object%20Reference))
  ;[1 1 1] 로비에서 나왔을 때 기존 세션 정보를 파기해 새로운 서버에 들어갈 수 있게 하기 위해 세션 파괴 정의
  (|DestroySession PlayerController))

(event Custom|NewPlayerCheck
  ;[1 1 1] 신규 플레이어면 기본 설정(캐릭터 설정, 닉네임)보여줌. 지금은 이 정보 게임에 저장하지만 나중엔 서버에 저장해야 할 것.
  (bind _returnvalue (SaveGame|DoesSaveGameExist (Variables|Default|GetPlayerSettingsSave)))
  (if _returnvalue
    (CallFunction|ShowMainMenu)
    (Variables|Default|SetisCreatedSaveFile true)
    (else
      (CallFunction|ShowOptionsMenu)
      (Variables|/Script/Engine.PlayerController|SetbShowMouseCursor (Game|GetPlayerController 0) true))))

(event Custom|ShowServerMenu
  ;[1 1 1] 서버 목록은 변수로 안 저장해서 누를 때 마다 새로 불러오게 함
  (bind _returnvalue (UserInterface|CreateWidget "/Game/UI/MainMenu/ServerMenu.ServerMenu_C" (Game|GetPlayerController 0)))
  (UserInterface|Viewport|AddtoViewport _returnvalue 0))

(event Custom|ShowHostMenu
  ;[1 1 1] 마우스는 메인 메뉴에서 보여주니까 여기선 설정 안 함
  (Utilities|IsValid (Variables|Widgets|GetHostMenuWB)
    (:Is%20Valid
      _)
    (:Is%20Not%20Valid
      (bind _returnvalue (UserInterface|CreateWidget "/Game/UI/MainMenu/HostMenu.HostMenu_C" (Game|GetPlayerController 0)))
      (Variables|Widgets|SetHostMenuWB _returnvalue)))
  (UserInterface|Viewport|AddtoViewport (Variables|Widgets|GetHostMenuWB) 0))

(event Custom|ShowOptionsMenu
  ;[1 1 1] 옵션 메뉴 표시
  (Utilities|IsValid (Variables|위젯|GetOptionsMenuWB)
    (:Is%20Valid
      _)
    (:Is%20Not%20Valid
      (bind _returnvalue (UserInterface|CreateWidget "/Game/UI/MainMenu/OptionsMenu.OptionsMenu_C" (Game|GetPlayerController 0)))
      (Variables|위젯|SetOptionsMenuWB _returnvalue)))
  (UserInterface|Viewport|AddtoViewport (Variables|위젯|GetOptionsMenuWB) 0))

(event Custom|ShowLoadingScreen
  ;[1 1 1] 로딩 스크린 출력
  (Utilities|IsValid (Variables|Widgets|GetLoadingScreenWB)
    (:Is%20Valid
      _)
    (:Is%20Not%20Valid
      (bind _returnvalue (UserInterface|CreateWidget "/Game/UI/AllLevels/LoadingScreen.LoadingScreen_C" (Game|GetPlayerController 0)))
      (Variables|Widgets|SetLoadingScreenWB _returnvalue)))
  (UserInterface|Viewport|AddtoViewport (Variables|Widgets|GetLoadingScreenWB) 0))

(event EventHandleNetworkError
  (params (FailureType :type ENetworkFailure%20Enum :default "NetDriverAlreadyExists") (bIsServer :type Boolean))
  ;[1 1 1] 네트워크 에러 처리 및 메세지 출력
  (if bIsServer
    _
    (else
      _))
  (Utilities|DisplayErrorMessage (CallFunction|NetErrortoString FailureType)))

(event EventHandleTravelError
  (params (FailureType :type ETravelFailure%20Enum :default "NoLevel"))
  ;[1 1 1] 트래블 에러 처리 및 메세지 출력
  (Utilities|DisplayErrorMessage (CallFunction|TravelErrortoString FailureType)))

(fn NetErrortoString
  (params (FailureType :type ENetworkFailure%20Enum :default "NetDriverAlreadyExists"))
  (return ""))

(fn TravelErrortoString
  (params (FailureType :type ETravelFailure%20Enum :default "NoLevel"))
  (return ""))